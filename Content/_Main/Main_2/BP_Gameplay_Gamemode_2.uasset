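; Multiplayer gameplay GameMode that runs a timed match and announces the top scorer or a tie.
; It spawns and registers joining player controllers, unpausing once their count matches MaxPlayers from the Steam GameInstance.
; Tick drives a Delay-gated one-second countdown pushed to every controller; at zero, a DoOnce compares character Puntos and broadcasts the result.
; Continuar calls FreePlay on all controllers; the custom pawn-spawning logic in SpawnDefaultPawnFor is disconnected.
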(event `self.ReceiveTick`
  (params (DeltaSeconds :type "Float (single-precision)"))
  (if (not (`self.Pause`))
    (`self.Timer`)))

(event `Timer`
  (bind _as_bp_gameplay_pc_2 (`self.As BP Gameplay PC 2`))
  (bind _bestscore (`self.BestScore`))
  (`KismetSystemLibrary.Delay` 1.0)
  (if (== (`self.Sec`) 0)
    (if (== (`self.Min`) 0)
      (`/Engine/EditorBlueprintResources/StandardMacros.DoOnce` false
        (:`Completed`
          (for _array_element _as_bp_gameplay_pc_2
            (bind _asthird_person_character (cast `/Game/ThirdPersonBP/Blueprints/ThirdPersonCharacter` (`Controller.K2_GetPawn` _array_element)))
            (bind _puntos (`/Game/ThirdPersonBP/Blueprints/ThirdPersonCharacter.Puntos` _asthird_person_character))
            (if (> _puntos _bestscore)
              (set `self.BestScore` _puntos)
              (set `self.NameWinner` (`|FormatText` "¿Quién ganó? : {name} " (`/Game/ThirdPersonBP/Blueprints/ThirdPersonCharacter.Player_Name` _asthird_person_character)))
              (elif (== _puntos _bestscore)
                (set `self.NameWinner` "Empate"))))
          (for _array_element_2 _as_bp_gameplay_pc_2
            (`/Game/_Main/Main_2/BP_Gameplay_PC_2.ShowWinner` _array_element_2 (`self.BestScore`) (`self.NameWinner`)))))
      (else
        (set `self.Sec` 59)
        (set `self.Min` (- (`self.Min`) 1))
        (for _array_element_3 _as_bp_gameplay_pc_2 :!label _label
          (`/Game/_Main/Main_2/BP_Gameplay_PC_2.Up_Timer` _array_element_3 (`self.Min`) (`self.Sec`)))))
    (else
      (set `self.Sec` (- (`self.Sec`) 1))
      (goto _label))))

(event `self.HandleStartingNewPlayer`
  (params (NewPlayer :type "PlayerController Object Reference"))
  (bind _as_bp_gameplay_pc_2 (`self.As BP Gameplay PC 2`))
  (`self.RestartPlayerAtPlayerStart` NewPlayer (`self.K2_FindPlayerStart` NewPlayer))
  (bind _game_instance (message `/Game/_Main/BP_GameIntance.Steam_GameInstance_Ref` (`GameplayStatics.GetGameInstance`)))
  (bind _asbp_gameplay_pc_2 (cast `/Game/_Main/Main_2/BP_Gameplay_PC_2` NewPlayer))
  (`KismetArrayLibrary.Array_Add` _as_bp_gameplay_pc_2 _asbp_gameplay_pc_2)
  (if (== (`/Game/_Main/Steam_GameIntance.Max_Players` _game_instance) (`KismetArrayLibrary.Array_Length` _as_bp_gameplay_pc_2))
    (`self.Start`)))

(event `Start`
  (set `self.Pause` false))

(event `Continuar`
  (for _array_element (`self.As BP Gameplay PC 2`)
    (`/Game/_Main/Main_2/BP_Gameplay_PC_2.Free_Play` _array_element)))

(fn `GamePlay_Ref_GM`
  (returns (GamePlay_GM :type "/Game/_Main/Main_2/BP_Gameplay_Gamemode_2 Object Reference"))
  (return self))

(fn `SpawnDefaultPawnFor`
  (params (NewPlayer :type "Controller Object Reference") (StartSpot :type "Actor Object Reference"))
  (returns (ReturnValue :type "Pawn Object Reference")))

(fn `UserConstructionScript`)