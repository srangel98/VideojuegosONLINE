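; Gameplay player controller that spawns and possesses the player's chosen character and manages match UI for a Steam session game.
; On local BeginPlay it reads character and name from the game instance, respawns the pawn at a random listed location and creates a timer seeded from the game mode.
; Events update the timer and show or dismiss the winner screen, switching input modes.
; A helper decrements lives, and EndPlay destroys the session.
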(event `Spawn_Each_Player`
  (params (Spawn_Char :type "/Game/ThirdPersonBP/Blueprints/ThirdPersonCharacter Class Reference") (Player_Name :type Text))
  (bind _returnvalue (`self.K2_GetPawn`))
  (bind _locations (`self.Locations`))
  (set `self.Location` (`|GetArrayItem` _locations (`KismetMathLibrary.RandomIntegerInRange` 0 (- (`KismetArrayLibrary.Array_Length` _locations) 1))))
  (`/Engine/EditorBlueprintResources/StandardMacros.IsValid` _returnvalue
    (:`Is Valid`
      (`self.K2_DestroyActor` _returnvalue))
    (:`Is Not Valid`
      _))
  (bind _returnvalue_2 (`|SpawnActorFromClass` Spawn_Char (`self.Location`) "Undefined" "OverrideRootScale" null null))
  (bind _output_get (set `/Game/ThirdPersonBP/Blueprints/ThirdPersonCharacter.Player_Name` Player_Name _returnvalue_2))
  (`self.Possess` _returnvalue_2))

(event `Get_Character_Class`
  (bind _output_get (set `self.Player Settings` (`/Game/_Main/Steam_GameIntance.Player_Info` (`self.Game Instance`))))
  (bind ((`Player_Name_4_9C9F73F64D73DA2D4E815C99697EEBBE` _player_name) (`Player_Character_24_04CFFAC94688F2C0E43D00841A956856` _player_character)) (break `/Game/_Main/Character/S_Players_Info` _output_get))
  (`self.Spawn_Each_Player` _player_character _player_name))

(event `self.ReceiveBeginPlay`
  (if (`self.IsLocalController`)
    (`WidgetLayoutLibrary.RemoveAllWidgets`)
    (bind _gameplay_gm (message `/Game/_Main/Main_2/BPI_GamePlayGM_2.GamePlay_Ref_GM` (`GameplayStatics.GetGameMode`)))
    (set `self.Game Play GM` _gameplay_gm)
    (bind _game_instance (message `/Game/_Main/BP_GameIntance.Steam_GameInstance_Ref` (`GameplayStatics.GetGameInstance`)))
    (set `self.Game Instance` _game_instance)
    (`self.Get_Character_Class`)
    (`self.Create_Wids`)))

(event `Create_Wids`
  (bind _game_play_gm (`self.Game Play GM`))
  (bind _returnvalue (`|CreateWidget` "/Game/_Main/Main_2/Timer.Timer_C" null (`/Game/_Main/Main_2/BP_Gameplay_Gamemode_2.Min` _game_play_gm) (`/Game/_Main/Main_2/BP_Gameplay_Gamemode_2.Sec` _game_play_gm)))
  (bind _output_get (set `self.Wid_Timer` _returnvalue))
  (`/Engine/EditorBlueprintResources/StandardMacros.IsValid` _output_get
    (:`Is Valid`
      (`UserWidget.AddToViewport` _output_get 0))))

(event `self.ReceiveEndPlay`
  (params (EndPlayReason :type "EEndPlayReason Enum" :default "Destroyed"))
  (message `/Game/_Main/BP_GameIntance.Destroy_Session` (`self.Game Instance`) self))

(event `Up_Timer`
  (params (Min :type Integer) (Sec :type Integer))
  (`/Game/_Main/Main_2/Timer.Upd_Timer` (`self.Wid_Timer`) Min Sec))

(event `ShowWinner`
  (params (Score :type Integer) (Name :type Text))
  (bind _returnvalue (`|CreateWidget` "/Game/_Main/Main_2/Winner.Winner_C" null Name (`|FormatText` "Su puntuación: {score}" (`KismetTextLibrary.Conv_IntToText` Score))))
  (bind _output_get (set `self.Wid_Win` _returnvalue))
  (`UserWidget.AddToViewport` _output_get 0)
  (`WidgetBlueprintLibrary.SetInputMode_UIOnlyEx` null _output_get)
  (set `self.bShowMouseCursor` true))

(event `Free_Play`
  (`WidgetBlueprintLibrary.SetInputMode_GameOnly` null)
  (`Widget.RemoveFromParent` (`self.Wid_Win`))
  (set `self.bShowMouseCursor` false))

(fn `Actualizar_Vidas`
  (returns (Murio :type Boolean))
  (locals (Murios :type Boolean :default true))
  (bind _returnvalue (- (`self.Vidas`) 1))
  (set `self.Vidas` _returnvalue)
  (bind _output_get (set `local.Murios` (<= _returnvalue 0)))
  (return _output_get))

(fn `GamePlay_Ref_PC`
  (returns (GamePlay_PC :type "/Game/_Main/Main_2/BP_Gameplay_PC_2 Object Reference"))
  (return self))

(fn `Set_Player_Setting`
  (returns (Output_Get :type "/Game/_Main/Character/S_Players_Info Structure"))
  (bind _game_instance (message `/Game/_Main/BP_GameIntance.Steam_GameInstance_Ref` (`GameplayStatics.GetGameInstance`)))
  (bind _output_get (set `self.Player Settings` (`/Game/_Main/Steam_GameIntance.Player_Info` _game_instance)))
  (return _output_get))

(fn `UserConstructionScript`
  (bind _game_instance (message `/Game/_Main/BP_GameIntance.Steam_GameInstance_Ref` (`GameplayStatics.GetGameInstance`)))
  (set `self.Player Settings` (`/Game/_Main/Steam_GameIntance.Player_Info` _game_instance)))