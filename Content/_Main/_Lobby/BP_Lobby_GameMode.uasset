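; Lobby game mode that tracks joining and leaving players and manages map selection, character pawns and match launch.
; PostLogin registers each lobby controller, marks the host ready and pulls server settings from the Steam game instance.
; Player lists and map choices are pushed to controllers through interface messages.
; Character changes respawn and possess pawns at a PlayerStart, and launch shows loading screens before server-traveling to the Battleflied level.
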(event `Update_Player_List`
  (bind _output_get (set `self.Current_Players` (`KismetArrayLibrary.Array_Length` (`self.As BP Lobby PC`))))
  (if (> _output_get 0)
    (`KismetArrayLibrary.Array_Clear` (`self.Connected_PLayers_Info`))
    (for _array_element (`self.As BP Lobby PC`)
      (bind _lobbygm (message `/Game/_Main/_Lobby/BP_Lobby_Interface.LobbyRef` _array_element))
      (`KismetArrayLibrary.Array_AddUnique` (`self.Connected_PLayers_Info`) (`/Game/_Main/_Lobby/BP_Lobby_PC.Player_Settings` _lobbygm))
      (`/Game/_Main/_Lobby/BP_Lobby_PC.Update_Num_Players` _array_element (`self.Current_Players`) (`self.Max Players`)))
    (`KismetSystemLibrary.Delay` 0.2)
    (for _array_element_2 (`self.As BP Lobby PC`)
      (bind _lobbygm_2 (message `/Game/_Main/_Lobby/BP_Lobby_Interface.LobbyRef` _array_element_2))
      (`/Game/_Main/_Lobby/BP_Lobby_PC.Update_Players_List` _lobbygm_2 (`self.Connected_PLayers_Info`)))))

(event `self.K2_PostLogin`
  (params (NewPlayer :type "PlayerController Object Reference"))
  (bind _as_bp_lobby_pc (`self.As BP Lobby PC`))
  (bind _outactors (`GameplayStatics.GetAllActorsOfClass` "/Script/Engine.PlayerStart"))
  (set `self.Spawner` _outactors)
  (set `self.Connected_Player` NewPlayer)
  (bind _asbp_lobby_pc (cast `/Game/_Main/_Lobby/BP_Lobby_PC` NewPlayer))
  (`KismetArrayLibrary.Array_AddUnique` _as_bp_lobby_pc _asbp_lobby_pc)
  (`KismetSystemLibrary.PrintString` (`KismetStringLibrary.Conv_IntToString` (`KismetArrayLibrary.Array_Length` _as_bp_lobby_pc)) true true (struct :`R` 0.212093 :`G` 1.0 :`A` 1.0) 5.0)
  (if (`Controller.IsLocalController` _asbp_lobby_pc)
    (bind _output_get (set `/Game/_Main/_Lobby/BP_Lobby_PC.Player_Settings` (make `/Game/_Main/Character/S_Players_Info` :`Player_Name` "Host" :`Is_Ready` true) _asbp_lobby_pc))
    (`KismetArrayLibrary.Array_Add` (`self.Connected_PLayers_Info`) _output_get)
    (else
      (`KismetArrayLibrary.Array_Add` (`self.Connected_PLayers_Info`) (`/Game/_Main/_Lobby/BP_Lobby_PC.Player_Settings` _asbp_lobby_pc))))
  (bind _game_instance (message `/Game/_Main/BP_GameIntance.Steam_GameInstance_Ref` (`GameplayStatics.GetGameInstance`)))
  (set `self.Server Name` (`/Game/_Main/Steam_GameIntance.Server_Name` _game_instance))
  (set `self.Max Players` (`/Game/_Main/Steam_GameIntance.Max_Players` _game_instance))
  (bind _lobbygm (message `/Game/_Main/_Lobby/BP_Lobby_Interface.LobbyRef` (`self.Connected_Player`)))
  (`/Game/_Main/_Lobby/BP_Lobby_PC.Initial_SetUp` _lobbygm (`self.Server Name`) (`self.Selected_Map_Img`) (`self.Selected_Map_Name`))
  (`KismetSystemLibrary.Delay` 0.5)
  (for _array_element (`self.As BP Lobby PC`)
    (`/Game/_Main/_Lobby/BP_Lobby_PC.Update_Players_List` _array_element (`self.Connected_PLayers_Info`))))

(event `Update_All`
  (bind _players (`self.Players`))
  (bind _output_get (set `self.Current_Players` (`KismetArrayLibrary.Array_Length` (`self.Players`))))
  (if (> _output_get 0)
    (`KismetArrayLibrary.Array_Clear` (`self.Connected_PLayers_Info`))
    (for _array_element _players
      (bind _lobbygm (message `/Game/_Main/_Lobby/BP_Lobby_Interface.LobbyRef` _array_element))
      (`KismetArrayLibrary.Array_AddUnique` (`self.Connected_PLayers_Info`) (`/Game/_Main/_Lobby/BP_Lobby_PC.Player_Settings` _lobbygm))
      (`/Game/_Main/_Lobby/BP_Lobby_PC.Update_Num_Players` _lobbygm (`self.Current_Players`) (`self.Max Players`)))
    (for _array_element_2 _players
      (bind _lobbygm_2 (message `/Game/_Main/_Lobby/BP_Lobby_Interface.LobbyRef` _array_element_2))
      (`/Game/_Main/_Lobby/BP_Lobby_PC.Update_Players_List` _lobbygm_2 (`self.Connected_PLayers_Info`)))
    (for _array_element_3 (`self.Connected_PLayers_Info`) :!label _label
      (if (== (`.Player_Character_24_04CFFAC94688F2C0E43D00841A956856` (break `/Game/_Main/Character/S_Players_Info` _array_element_3)) null)
        (set `self.Can_Start` false)
        (`self.Cant_Start`)
        (else
          (set `self.Can_Start` true))))))

(event `Cant_Start`
  (goto _label :!via `Break`))

(event `Start_Loading_Screen`
  (for _array_element (`self.As BP Lobby PC`)
    (bind _lobbygm (message `/Game/_Main/_Lobby/BP_Lobby_Interface.LobbyRef` _array_element))
    (`/Game/_Main/_Lobby/BP_Lobby_PC.Show_Loading_S` _lobbygm))
  (`self.Launch_Game`))

(event `Host_Update_Game`
  (params (Selected_Map_Img :type "Texture2D Object Reference") (Selected_Map_Name :type Text) (Selected_Map_Time :type Text) (Selected_Map_ID :type Integer))
  (set `self.Selected_Map_Img` Selected_Map_Img)
  (set `self.Selected_Map_Name` Selected_Map_Name)
  (set `self.Selected_Map_Time` Selected_Map_Time)
  (set `self.Selected_Map_ID` Selected_Map_ID)
  (for _array_element (`self.As BP Lobby PC`)
    (bind _lobbygm (message `/Game/_Main/_Lobby/BP_Lobby_Interface.LobbyRef` _array_element))
    (`/Game/_Main/_Lobby/BP_Lobby_PC.Update_Lobby_Settings` _lobbygm (`self.Selected_Map_Img`) (`self.Selected_Map_Name`))))

(event `self.K2_OnLogout`
  (params (ExitingController :type "Controller Object Reference"))
  (bind _as_bp_lobby_pc (`self.As BP Lobby PC`))
  (for (_array_element _array_index) _as_bp_lobby_pc
    (if (== _array_element ExitingController)
      (break)))
  (`KismetArrayLibrary.Array_Remove` _as_bp_lobby_pc _array_index)
  (`KismetArrayLibrary.Array_Remove` (`self.Connected_PLayers_Info`) _array_index)
  (`self.Update_Player_List`))

(event `Launch_Game`
  (switch `int` (`self.Selected_Map_ID`)
    (:`0`
      _)
    (:`1`
      _))
  (`KismetSystemLibrary.ExecuteConsoleCommand` "servertravel /Game/Level/Battleflied" (`GameplayStatics.GetPlayerController` 0)))

(event `Change_Char`
  (params (Target :type "PlayerController Object Reference") (Character :type "Character Class Reference") (`Change?` :type Boolean))
  (bind _returnvalue (`Controller.K2_GetPawn` Target))
  (bind _spawner (`self.Spawner`))
  (if (not `Change?`)
    (`/Engine/EditorBlueprintResources/StandardMacros.IsValid` _returnvalue
      (:`Is Valid`
        (`self.K2_DestroyActor` _returnvalue))
      (:`Is Not Valid`
        _))
    (bind _returnvalue_2 (`|SpawnActorFromClass` Character (`self.GetTransform` (`|GetArrayItem` _spawner (- (`KismetArrayLibrary.Array_Length` _spawner) 1))) "AlwaysSpawn" "OverrideRootScale" null null))
    (`Controller.Possess` Target _returnvalue_2)))

(fn `LobbyGMRef`
  (returns (LobbyGM :type "/Game/_Main/_Lobby/BP_Lobby_GameMode Object Reference"))
  (return self))

(fn `LobbyRef`
  (returns (LobbyGM :type "/Game/_Main/_Lobby/BP_Lobby_PC Object Reference"))
  (return null))

(fn `UserConstructionScript`)