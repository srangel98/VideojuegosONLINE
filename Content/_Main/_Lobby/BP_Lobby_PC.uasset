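; Lobby player controller that runs each player's lobby menu, ready state and character selection in a multiplayer session.
; It creates the lobby widget, refreshes map, player count and list, then swaps to a loading screen; EndPlay destroys the session.
; PlayerSettings changes reach the lobby GameMode through interface messages, which refresh the player list.
; Character changes respawn and repossess the pawn, storing the choice in the Steam GameInstance; client-widget and save calls are disconnected.
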(event `Initial_SetUp`
  (params (ServerName :type Text) (Map_Image :type "Texture2D Object Reference") (Map_Name :type Text))
  (`self.SetUp_Lobby_Menu` ServerName)
  (`KismetSystemLibrary.Delay` 0.2)
  (`self.Update_Lobby_Settings` Map_Image Map_Name)
  (`KismetSystemLibrary.Delay` 0.2)
  (`self.Call_Update` (`self.Player_Settings`)))

(event `SetUp_Lobby_Menu`
  (params (ServerName :type Text))
  (set `self.bShowMouseCursor` true)
  (bind _returnvalue (`|CreateWidget` "/Game/_Main/_Lobby/Wid_Lobby_Menu.Wid_Lobby_Menu_C" null ServerName))
  (bind _output_get (set `self.Wid_Lobby` _returnvalue))
  (`UserWidget.AddToViewport` _output_get 0))

(event `Update_Num_Players`
  (params (Current_Payers :type Integer) (Max_Players :type Integer))
  ;[1 1 1] Players_List_Events
  (`/Game/_Main/_Lobby/Wid_Lobby_Menu.Update_Display` (`self.Wid_Lobby`) (`|FormatText` "{Current Players} / {Max}" (`KismetTextLibrary.Conv_IntToText` Current_Payers) (`KismetTextLibrary.Conv_IntToText` Max_Players))))

(event `Update_Lobby_Settings`
  (params (Map_Image :type "Texture2D Object Reference") (Map_Name :type Text))
  (`/Game/_Main/_Lobby/Wid_Lobby_Menu.Update_Lobby_Info` (`self.Wid_Lobby`) Map_Image Map_Name))

(event `Update_Players_List`
  (params (List :type "Array of /Game/_Main/Character/S_Players_Info Structure"))
  ;[1 1 1] Players_List_Events
  (set `self.All_Connected_Players` List)
  (`KismetSystemLibrary.Delay` 0.1)
  (`self.Wid_Lobby`
    (:`then`
      (`/Game/_Main/_Lobby/Wid_Lobby_Menu.Update_Player_List` (`self.Wid_Lobby`) (`self.All_Connected_Players`)))
    (:`else`)))

(event `Call_Update`
  (params (`Players Info` :type "/Game/_Main/Character/S_Players_Info Structure") (`Changed Status` :type Boolean) (Char_to_See :type "Character Class Reference"))
  (bind _output_get (set `self.Player_Settings` `Players Info`))
  (bind _lobbygm (message `/Game/_Main/_Lobby/BP_Lobby_GM.LobbyGMRef` (`GameplayStatics.GetGameMode`)))
  (`/Game/_Main/_Lobby/BP_Lobby_GameMode.Change_Char` _lobbygm self Char_to_See `Changed Status`)
  (`/Game/_Main/_Lobby/BP_Lobby_GameMode.Update_Player_List` _lobbygm))

(event `Players_Ready`
  (params (PI :type "/Game/_Main/Character/S_Players_Info Structure"))
  ;[1 1 1] Players_List_Events
  (bind _output_get (set `self.Player_Settings` PI))
  (setmembers `/Game/_Main/Character/S_Players_Info` :`StructRef` _output_get :`Is_Ready` (not (`.Is_Ready_22_0FBDD1CB4D939BE1132B12B22B71F19E` (break `/Game/_Main/Character/S_Players_Info` _output_get))))
  (bind _lobbygm (message `/Game/_Main/_Lobby/BP_Lobby_GM.LobbyGMRef` (`GameplayStatics.GetGameMode`)))
  (`/Game/_Main/_Lobby/BP_Lobby_GameMode.Update_Player_List` _lobbygm))

(event `Show_Loading_S`
  (`Widget.RemoveFromParent` (`self.Wid_Lobby`))
  (bind _returnvalue (`|CreateWidget` "/Game/_Main/Wid_LoadingScreen.Wid_LoadingScreen_C" self))
  (`UserWidget.AddToViewport` _returnvalue 0))

(event `self.ReceiveEndPlay`
  (params (EndPlayReason :type "EEndPlayReason Enum" :default "Destroyed"))
  (`DestroySessionCallbackProxy.DestroySession` self))

(event `Assing_Char`
  (params (Selected_Char :type Integer) (Character_IMG :type "Texture2D Object Reference"))
  (set `self.Character_IMG` Character_IMG)
  (set `self.Selected Char` Selected_Char)
  (`self.Charr`))

(event `Charr`
  (bind _lobbygm (message `/Game/_Main/_Lobby/BP_Lobby_GM.LobbyGMRef` (`GameplayStatics.GetGameMode`)))
  (`self.Assing_Player` (`self.Character_IMG`) (`|GetArrayItem` (`/Game/_Main/_Lobby/BP_Lobby_GameMode.Characters` _lobbygm) (`self.Selected Char`))))

(event `Assing_Player`
  (params (Character_Image :type "Texture2D Object Reference") (Player_Character :type "Character Class Reference") (Seen_Char :type "Character Class Reference"))
  (bind _structout (setmembers `/Game/_Main/Character/S_Players_Info` :`StructRef` (`self.Player_Settings`) :`Player_Character` null :`Character_Image` Character_Image))
  (`self.Call_Update` _structout false Seen_Char))

(event `Up_Char`
  (params (Char_Class_Show :type "/Game/ThirdPersonBP/Blueprints/ThirdPersonCharacter_Show Class Reference") (Char_Class2 :type "/Game/ThirdPersonBP/Blueprints/ThirdPersonCharacter Class Reference"))
  (bind _returnvalue (`self.K2_GetPawn`))
  (set `self.Transform` (`self.GetTransform` _returnvalue))
  (`self.K2_DestroyActor` _returnvalue)
  (bind _returnvalue_2 (`|SpawnActorFromClass` Char_Class_Show (`self.Transform`) "AlwaysSpawn" "OverrideRootScale" null null))
  (`self.Possess` _returnvalue_2)
  (bind _game_instance (message `/Game/_Main/BP_GameIntance.Steam_GameInstance_Ref` (`GameplayStatics.GetGameInstance`)))
  (set `/Game/_Main/Steam_GameIntance.Chosen_Character` Char_Class2 _game_instance))

(event `Set_Char_Class`
  (params (Char_Class :type "/Game/ThirdPersonBP/Blueprints/ThirdPersonCharacter Class Reference"))
  (bind _game_instance (message `/Game/_Main/BP_GameIntance.Steam_GameInstance_Ref` (`GameplayStatics.GetGameInstance`)))
  (bind _structout (setmembers `/Game/_Main/Character/S_Players_Info` :`StructRef` (`self.Player_Settings`) :`Player_Character` Char_Class))
  (set `/Game/_Main/Steam_GameIntance.Chosen_Character` Char_Class _game_instance)
  (`self.Call_Update` _structout true))

(event `Save_Game`
  (`self.Save_S`
    (:`then`
      (set `/Game/_Main/Save_Game.Player_Info` (`self.Player_Settings`) (stale _output_get))
      (`GameplayStatics.SaveGameToSlot` (stale _output_get) (`self.Player_Slot Name`)))
    (:`else`
      (bind _returnvalue (`GameplayStatics.CreateSaveGameObject` "/Game/_Main/Save_Game.Save_Game_C"))
      (bind _output_get (set `self.Save_S` _returnvalue)))))

(fn `LobbyRef`
  (returns (LobbyGM :type "/Game/_Main/_Lobby/BP_Lobby_PC Object Reference"))
  (return self))

(fn `UserConstructionScript`)