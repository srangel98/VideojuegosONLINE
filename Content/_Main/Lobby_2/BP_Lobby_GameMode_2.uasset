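; BP_Lobby_GameMode_2 is the multiplayer lobby game mode that tracks connected players and launches the match.
; Logins and logouts update controller and player-info arrays, then push player counts and lists to every controller, marking the first player ready.
; Host map settings are relayed to all controllers, and starting shows loading screens before server-travelling to Battlefield or Mansion by map ID.
; The character-selection start check is disconnected.
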(event `Update_All_Players`
  (bind _connected_player_info (`self.Connected_Player_Info`))
  (bind _output_get (set `self.Current_Players` (`KismetArrayLibrary.Array_Length` (`self.All_Connected_Players`))))
  (if (> _output_get 0)
    (`KismetArrayLibrary.Array_Clear` (`self.Connected_Player_Info`))
    (for (_array_element _array_index) (`self.All_Connected_Players`)
      (bind _lobby_pc (message `/Game/_Main/Lobby_2/BPI_Lobby_PC_2.LobbyRef` _array_element))
      (if (== _array_index 0)
        (bind _structout (setmembers `/Game/_Main/Character/S_Players_Info` :`StructRef` (`/Game/_Main/Lobby_2/BP_Lobby_PC_2.Player_Info` _lobby_pc) :`Is_Ready` true))
        (`KismetArrayLibrary.Array_AddUnique` _connected_player_info _structout)
        (else
          (`KismetArrayLibrary.Array_AddUnique` _connected_player_info (`/Game/_Main/Lobby_2/BP_Lobby_PC_2.Player_Info` _lobby_pc))))
      (`/Game/_Main/Lobby_2/BP_Lobby_PC_2.Update_Num_Players` _lobby_pc (`self.Current_Players`) (`self.Max Players`)))
    (`KismetSystemLibrary.Delay` 0.5)
    (for _array_element_2 (`self.All_Connected_Players`)
      (bind _lobby_pc_2 (message `/Game/_Main/Lobby_2/BPI_Lobby_PC_2.LobbyRef` _array_element_2))
      (`/Game/_Main/Lobby_2/BP_Lobby_PC_2.Update_Player_Lists` _lobby_pc_2 (`self.Connected_Player_Info`)))))

(event `self.K2_OnLogout`
  (params (ExitingController :type "Controller Object Reference"))
  (bind _all_connected_players (`self.All_Connected_Players`))
  (for (_array_element _array_index) _all_connected_players
    (if (== ExitingController _array_element)
      (break)))
  (`KismetArrayLibrary.Array_Remove` _all_connected_players _array_index)
  (`KismetArrayLibrary.Array_Remove` (`self.Connected_Player_Info`) _array_index)
  (`self.Update_All_Players`))

(event `Cant_S`
  (for _array_element (`self.Connected_Player_Info`) :!via `Break`
    (if (== (`.Player_Character_24_04CFFAC94688F2C0E43D00841A956856` (break `/Game/_Main/Character/S_Players_Info` _array_element)) null)
      (set `self.Can_Start` false)
      (`self.Cant_S`)
      (else
        (set `self.Can_Start` true)))))

(event `self.K2_PostLogin`
  (params (NewPlayer :type "PlayerController Object Reference"))
  (set `self.Player_C` NewPlayer)
  (bind _asbp_lobby_pc_2 (cast `/Game/_Main/Lobby_2/BP_Lobby_PC_2` NewPlayer))
  (`KismetArrayLibrary.Array_AddUnique` (`self.All_Connected_Players`) _asbp_lobby_pc_2)
  (`KismetArrayLibrary.Array_AddUnique` (`self.Connected_Player_Info`) (`/Game/_Main/Lobby_2/BP_Lobby_PC_2.Player_Info` _asbp_lobby_pc_2))
  (bind _game_instance (message `/Game/_Main/BP_GameIntance.Steam_GameInstance_Ref` (`GameplayStatics.GetGameInstance`)))
  (set `self.Max Players` (`/Game/_Main/Steam_GameIntance.Max_Players` _game_instance))
  (`KismetSystemLibrary.Delay` 0.5)
  (bind _lobby_pc (message `/Game/_Main/Lobby_2/BPI_Lobby_PC_2.LobbyRef` (`self.Player_C`)))
  (`/Game/_Main/Lobby_2/BP_Lobby_PC_2.Init` _lobby_pc)
  (`self.Update_All_Players`)
  (`KismetSystemLibrary.Delay` 0.5)
  (for _array_element (`self.All_Connected_Players`)
    (`/Game/_Main/Lobby_2/BP_Lobby_PC_2.Update_Player_Lists` _array_element (`self.Connected_Player_Info`))))

(event `Start_Loading_S`
  (for _array_element (`self.All_Connected_Players`)
    (`/Game/_Main/Lobby_2/BP_Lobby_PC_2.Show_Loading_S` _array_element))
  (`self.Launch_Game`))

(event `Launch_Game`
  (bind _returnvalue (`GameplayStatics.GetPlayerController` 0))
  (switch `int` (`self.Map_ID`)
    (:`0`
      (`KismetSystemLibrary.ExecuteConsoleCommand` "servertravel/Game/Level/Battleflied" _returnvalue))
    (:`1`
      (`KismetSystemLibrary.ExecuteConsoleCommand` "servertravel/Game/Level/Mansion" _returnvalue))))

(event `Host_Act_Game_Setting`
  (params (Map_Name :type Text) (Map_ID :type Integer) (Map_Image :type "Texture2D Object Reference") (Map_Desc :type Text))
  (set `self.Map_Desc` Map_Desc)
  (set `self.Map_Name` Map_Name)
  (set `self.Map_ID` Map_ID)
  (set `self.Map_Image` Map_Image)
  (for _array_element (`self.All_Connected_Players`)
    (`/Game/_Main/Lobby_2/BP_Lobby_PC_2.Update_Each_Lobby_S` _array_element (`self.Map_Name`) (`self.Map_Image`) (`self.Map_ID`) (`self.Map_Desc`))))

(fn `LobbyGMRef`
  (returns (Lobby_GM :type "/Game/_Main/Lobby_2/BP_Lobby_GameMode_2 Object Reference"))
  (return self))

(fn `UserConstructionScript`)