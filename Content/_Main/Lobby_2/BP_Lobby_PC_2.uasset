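; Lobby player controller that manages each player's menu, character choice and ready state before a match.
; It takes player info from the Steam game instance, saves it to a save slot and asks the lobby game mode to refresh all players.
; Update events feed player list, count and map info to the lobby widget, swap the previewed pawn or show a loading screen.
; EndPlay tells the game instance to destroy the session.
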(event `Init`
  ;[1 1 1] Prueba_2
  (`self.Save_Info`))

(event `self.ReceiveBeginPlay`
  ;[1 1 1] Prueba_2
  (bind _game_instance (message `/Game/_Main/BP_GameIntance.Steam_GameInstance_Ref` (`GameplayStatics.GetGameInstance`)))
  (bind _output_get (set `self.Game Instance` _game_instance))
  (set `self.Player_Info` (`/Game/_Main/Steam_GameIntance.Player_Info` _output_get))
  (`self.Create_Wid`))

(event `Create_Wid`
  ;[1 1 1] Prueba_2
  (bind _returnvalue (`|CreateWidget` "/Game/_Main/Lobby_2/Wid_Lobby_Menu_2.Wid_Lobby_Menu_2_C"))
  (bind _output_get (set `self.Wid_Lobby` _returnvalue))
  (`UserWidget.AddToViewport` _output_get 0))

(event `Call_Update`
  (params (Player_Info :type "/Game/_Main/Character/S_Players_Info Structure"))
  ;[1 1 1] Prueba_2
  (set `self.Player_Info` Player_Info)
  (bind _lobby_gm (message `/Game/_Main/Lobby_2/BPI_Lobby_GM_2.LobbyGMRef` (`GameplayStatics.GetGameMode`)))
  (`/Game/_Main/Lobby_2/BP_Lobby_GameMode_2.Update_All_Players` _lobby_gm))

(event `Update_Player_Lists`
  (params (Players_Info :type "Array of /Game/_Main/Character/S_Players_Info Structure"))
  ;[1 1 1] Prueba_2
  (set `self.Lis_Players Info` Players_Info)
  (`KismetSystemLibrary.Delay` 0.2)
  (bind _wid_lobby (`self.Wid_Lobby`)
    (:`then`
      (`/Game/_Main/Lobby_2/Wid_Lobby_Menu_2.Update_Player_List_Wid` _wid_lobby (`self.Lis_Players Info`)))
    (:`else`)))

(event `Change_Character_View`
  (params (`New Character` :type "/Game/ThirdPersonBP/Blueprints/ThirdPersonCharacter Class Reference") (Seen_Char :type "/Game/ThirdPersonBP/Blueprints/ThirdPersonCharacter_Show Class Reference"))
  (bind _returnvalue (`self.K2_GetPawn`))
  ;[1 1 1] Prueba_2
  (set `self.Spawn_Transform` (`self.GetTransform` _returnvalue))
  (`self.K2_DestroyActor` _returnvalue)
  (bind _returnvalue_2 (`|SpawnActorFromClass` Seen_Char (`self.Spawn_Transform`) "Undefined" "OverrideRootScale" null null))
  (`self.Possess` _returnvalue_2))

(event `Set_Character_Class`
  (params (Player_Info :type "/Game/_Main/Character/S_Players_Info Structure"))
  ;[1 1 1] Prueba_2
  (set `self.Player_Info` Player_Info)
  (bind _game_instance (message `/Game/_Main/BP_GameIntance.Steam_GameInstance_Ref` (`GameplayStatics.GetGameInstance`)))
  (set `/Game/_Main/Steam_GameIntance.Player_Info` (`self.Player_Info`) _game_instance))

(event `Assing_Char`
  (params (Player_Character :type "/Game/ThirdPersonBP/Blueprints/ThirdPersonCharacter Class Reference"))
  ;[1 1 1] Prueba_2
  (bind _structout (setmembers `/Game/_Main/Character/S_Players_Info` :`StructRef` (`self.Player_Info`) :`Player_Character` Player_Character))
  (`self.Save_Info`)
  (`self.Call_Update` _structout))

(event `Show_Loading_S`
  ;[1 1 1] Prueba_2
  (`Widget.RemoveFromParent` (`self.Wid_Lobby`))
  (bind _returnvalue (`|CreateWidget` "/Game/_Main/Wid_LoadingScreen.Wid_LoadingScreen_C" self))
  (`UserWidget.AddToViewport` _returnvalue 0))

(event `Update_Num_Players`
  (params (Current_Payers :type Integer) (Max_Players :type Integer))
  ;[1 1 1] Prueba_2
  (`/Game/_Main/Lobby_2/Wid_Lobby_Menu_2.Update_Players` (`self.Wid_Lobby`) (`|FormatText` "{Current Players} / {Max}" (`KismetTextLibrary.Conv_IntToText` Current_Payers) (`KismetTextLibrary.Conv_IntToText` Max_Players))))

(event `Update_Each_Lobby_S`
  (params (Map_Name_T :type Text) (Map_Image :type "Texture2D Object Reference"))
  ;[1 1 1] Prueba_2
  (`/Game/_Main/Lobby_2/Wid_Lobby_Menu_2.Update_Info` (`self.Wid_Lobby`) Map_Name_T Map_Image))

(event `Save_Info`
  ;[1 1 1] Prueba_2
  (`self.Save_Slot`
    (:`then`
      _)
    (:`else`
      (bind _returnvalue (`GameplayStatics.CreateSaveGameObject` "/Game/_Main/Save_Game.Save_Game_C"))
      (bind _output_get (set `self.Save_Slot` _returnvalue))))
  (set `/Game/_Main/Save_Game.Player_Info` (`self.Player_Info`) _output_get)
  (`GameplayStatics.SaveGameToSlot` _output_get (`self.Players_Info`)))

(event `Player_Ready`
  (params (Player_Info :type "/Game/_Main/Character/S_Players_Info Structure"))
  ;[1 1 1] Prueba_2
  (bind _output_get (set `self.Player_Info` Player_Info))
  (setmembers `/Game/_Main/Character/S_Players_Info` :`StructRef` _output_get :`Is_Ready` (not (`.Is_Ready_22_0FBDD1CB4D939BE1132B12B22B71F19E` (break `/Game/_Main/Character/S_Players_Info` _output_get))))
  (bind _lobby_gm (message `/Game/_Main/Lobby_2/BPI_Lobby_GM_2.LobbyGMRef` (`GameplayStatics.GetGameMode`)))
  (`/Game/_Main/Lobby_2/BP_Lobby_GameMode_2.Update_All_Players` _lobby_gm))

(event `Load_Info`
  (for _ (`self.Lis_Players Info`)
    (bind _returnvalue (`GameplayStatics.LoadGameFromSlot` (`self.Players_Info`)))
    (bind _assave_game (cast `/Game/_Main/Save_Game` _returnvalue)
      (:`then`
        (`KismetSystemLibrary.PrintString` (`KismetSystemLibrary.GetClassDisplayName` (`.Player_Character_24_04CFFAC94688F2C0E43D00841A956856` (break `/Game/_Main/Character/S_Players_Info` (`/Game/_Main/Save_Game.Player_Info` _assave_game))))))
      (:`CastFailed`
        (`KismetSystemLibrary.PrintString` "Hello")))))

(event `self.ReceiveEndPlay`
  (params (EndPlayReason :type "EEndPlayReason Enum" :default "Destroyed"))
  (message `/Game/_Main/BP_GameIntance.Destroy_Session` (`self.Game Instance`) self))

(fn `LobbyRef`
  (returns (Lobby_PC :type "/Game/_Main/Lobby_2/BP_Lobby_PC_2 Object Reference"))
  (return self))

(fn `UserConstructionScript`)