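; Gameplay player controller that gets the player spawned as their selected character and connects them to in-game chat.
; On local BeginPlay it clears widgets, passes PlayerSettings through PassInfoServer for the game mode to spawn the character, then triggers chat widget setup after a delay.
; Chat messages go to the game mode tagged with the player's name.
; Interface-style getters reach the game mode and Steam game instance, and expose the controller itself.
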(event `Get_Char_Class`
  (bind _game_instance (message `/Game/_Main/BP_GameIntance.Steam_GameInstance_Ref` (`GameplayStatics.GetGameInstance`)))
  (set `self.Char Class` (`/Game/_Main/Steam_GameIntance.Char_Class` _game_instance)))

(event `self.ReceiveBeginPlay`
  (if (`self.IsLocalController`)
    (`WidgetLayoutLibrary.RemoveAllWidgets`)
    (`KismetSystemLibrary.Delay` 0.2)
    (`self.Pass_Info_Server` (`self.Player_Settings`))
    (`WidgetBlueprintLibrary.SetInputMode_GameOnly` self)))

(event `Pass_Info_Server`
  (params (Player_Settings :type "/Game/_Main/Character/S_Players_Info Structure"))
  (bind _output_get (set `self.Player_Settings` Player_Settings))
  (bind _gameplay_gm (message `/Game/_Main/_GamePlay/BPI_GamePlayGM.GamePlay_Ref_GM` (`GameplayStatics.GetGameMode`)))
  (`/Game/_Main/_GamePlay/BP_Gameplay_Gamemode.Spawn_Player` _gameplay_gm self (`.Player_Character_19_04CFFAC94688F2C0E43D00841A956856` (break `/Game/_Main/Character/S_Players_Info` _output_get)))
  (`KismetSystemLibrary.Delay` 0.5)
  (`self.SetUp_UI`))

(event `SetUp_UI`
  (bind _returnvalue (`|CreateWidget` "/Game/_Main/_Lobby/Wid_Chat_GamePlay.Wid_Chat_GamePlay_C"))
  (bind _output_get (set `self.Game_Chat_Wid` _returnvalue))
  (`UserWidget.AddToViewport` _output_get 0))

(event `Get_Chat_Message`
  (params (Text :type Text))
  (set `self.Text` Text)
  (set `self.Sender` (`.Player_Name_4_9C9F73F64D73DA2D4E815C99697EEBBE` (break `/Game/_Main/Character/S_Players_Info` (`self.Player_Settings`))))
  (bind _gameplay_gm (message `/Game/_Main/_GamePlay/BPI_GamePlayGM.GamePlay_Ref_GM` (`GameplayStatics.GetGameMode`)))
  (`/Game/_Main/_GamePlay/BP_Gameplay_Gamemode.Update_Chat` _gameplay_gm (`self.Sender`) (`self.Text`)))

(fn `GamePlay_Ref_PC`
  (returns (GamePlay_PC :type "/Game/_Main/_GamePlay/BP_Gameplay_PC Object Reference"))
  (return self))

(fn `UserConstructionScript`)