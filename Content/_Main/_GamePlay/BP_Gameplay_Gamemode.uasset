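; Multiplayer gameplay Game Mode that spawns player characters and tracks their controllers.
; Default pawn spawning asks each controller for its chosen character class, while Spawn_Player spawns and possesses a selected class at a random PlayerStart.
; Controller swaps add the new controller to AllPlayers, and logout tells the Steam game instance to destroy the session for the exiting controller.
; Cross-class references go through message calls, with the Game Mode returning itself as a reference.
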(event `self.HandleStartingNewPlayer`
  (params (NewPlayer :type "PlayerController Object Reference"))
  (`self.RestartPlayerAtPlayerStart` NewPlayer (`self.K2_FindPlayerStart` NewPlayer)))

(event `Spawn_Player`
  (params (Player_C :type "PlayerController Object Reference") (Chracter_Select :type "Character Class Reference"))
  (bind _spawn_points (`self.Spawn_Points`))
  (bind _outactors (`GameplayStatics.GetAllActorsOfClass` "/Script/Engine.PlayerStart"))
  (set `self.Spawn_Points` _outactors)
  (`/Engine/EditorBlueprintResources/StandardMacros.IsValid` (`Controller.K2_GetPawn` Player_C)
    (:`Is Valid`
      (`self.K2_DestroyActor`))
    (:`Is Not Valid`
      _))
  (bind _returnvalue (`|SpawnActorFromClass` Chracter_Select (`self.GetTransform` (`|GetArrayItem` _spawn_points (`KismetMathLibrary.RandomIntegerInRange` 0 (- (`KismetArrayLibrary.Array_Length` _spawn_points) 1)))) "AlwaysSpawn" "OverrideRootScale" null null))
  (`Controller.Possess` Player_C _returnvalue))

(event `self.K2_OnSwapPlayerControllers`
  (params (OldPC :type "PlayerController Object Reference") (NewPC :type "PlayerController Object Reference"))
  (`KismetArrayLibrary.Array_Add` (`self.All_Players`) NewPC))

(event `self.K2_OnLogout`
  (params (ExitingController :type "Controller Object Reference"))
  (bind _gameplay_pc (message `/Game/_Main/_GamePlay/BPI_GamePlayPC.GamePlay_Ref_PC` ExitingController))
  (bind _game_instance (message `/Game/_Main/BP_GameIntance.Steam_GameInstance_Ref` (`GameplayStatics.GetGameInstance`)))
  (message `/Game/_Main/BP_GameIntance.Destroy_Session` _game_instance _gameplay_pc))

(fn `GamePlay_Ref_GM`
  (returns (GamePlay_GM :type "/Game/_Main/_GamePlay/BP_Gameplay_Gamemode Object Reference"))
  (return self))

(fn `GamePlay_Ref_PC`
  (returns (GamePlay_PC :type "/Game/_Main/_GamePlay/BP_Gameplay_PC Object Reference"))
  (return null))

(fn `SpawnDefaultPawnFor`
  (params (NewPlayer :type "Controller Object Reference") (StartSpot :type "Actor Object Reference"))
  (returns (ReturnValue :type "Pawn Object Reference"))
  (bind _gameplay_pc (message `/Game/_Main/_GamePlay/BPI_GamePlayPC.GamePlay_Ref_PC` NewPlayer))
  (`/Game/_Main/_GamePlay/BP_Gameplay_PC.Get_Char_Class` _gameplay_pc)
  (bind _returnvalue (`|SpawnActorFromClass` (`/Game/_Main/_GamePlay/BP_Gameplay_PC.Char Class` _gameplay_pc) (`self.GetTransform` StartSpot) "Undefined" "OverrideRootScale" null null))
  (return _returnvalue))

(fn `UserConstructionScript`)