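; Player bow that charges, fires and reloads normal, electric or ice arrows.
; A timeline drives ChargeAmount, with a separate curve for electric shots, and reverses when charging ends.
; Reload events spawn an arrow on the bow mesh's Flechas socket, with the elemental variants first destroying any loaded arrow.
; Fire detaches the arrow, launches it with the charge and direction, then clears the reference and stops charging.
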(event `Begin_Charge`
  (params (Electrico :type Boolean))
  (`self.Flechas`
    (:`then`
      (bind (_direction _chague_amount _chargue_amount_power) (`Timeline|Chargue_Bow` :!label _label)
        (:`Update`
          (if Electrico
            (set `self.Charge_Amount` _chargue_amount_power)
            (else
              (set `self.Charge_Amount` _chague_amount))))))
    (:`else`)))

(event `Stop_Charge`
  (`|ExecutionSequence`
    (:`then_0`
      (goto _label :!via `Stop`))
    (:`then_1`
      (goto _label :!via `SetNewTime`))))

(event `End_Charge`
  (`self.Flechas`
    (:`then`
      (goto _label :!via `Reverse`))
    (:`else`)))

(event `Fire`
  (params (Direccion :type "Vector Structure"))
  (bind _flechas (`self.Flechas`)
    (:`then`
      (`self.K2_DetachFromActor` _flechas "KeepWorld" "KeepWorld" "KeepWorld")
      (`/Game/FirstPersonBP/Blueprints/Flechas.Fire` (`self.Flechas`) (`self.Charge_Amount`) Direccion)
      (set `self.Flechas` null)
      (`self.Stop_Charge`))
    (:`else`)))

(event `Reload`
  (params (Character :type "Actor Object Reference") (Is_Electric :type Boolean))
  (if Is_Electric
    (bind _returnvalue (`|SpawnActorFromClass` "/Game/FirstPersonBP/Blueprints/Flechas_Electricas.Flechas_Electricas_C" (`KismetMathLibrary.MakeTransform` (0.0 0.0 0.0)) "Undefined" "OverrideRootScale" Character "NewEnumerator2" null :!label _label_2))
    (bind _output_get (set `self.Flechas` _returnvalue))
    (else
      (bind _returnvalue_2 (`|SpawnActorFromClass` "/Game/FirstPersonBP/Blueprints/Flechas.Flechas_C" (`KismetMathLibrary.MakeTransform` (0.0 0.0 0.0)) "Undefined" "OverrideRootScale" Character "NewEnumerator2" null))
      (bind _output_get_2 (set `self.Flechas` _returnvalue_2))))
  (`self.K2_AttachToComponent` _output_get (`self.Bow`) "Flechas" "KeepRelative" "KeepRelative" "KeepRelative" true)
  (`self.K2_AttachToComponent` _output_get_2 (`self.Bow`) "Flechas" "KeepRelative" "KeepRelative" "KeepRelative" true))

(event `Reload_con_Electric`
  (bind _flechas (`self.Flechas`)
    (:`then`
      (`self.K2_DestroyActor` _flechas)
      (goto _label_2))
    (:`else`)))

(event `Reload_con_Hielo`
  (params (Character :type "/Game/ThirdPersonBP/Blueprints/ThirdPersonCharacter Object Reference"))
  (bind _flechas (`self.Flechas`)
    (:`then`
      (`self.K2_DestroyActor` _flechas)
      (bind _returnvalue (`|SpawnActorFromClass` "/Game/FirstPersonBP/Blueprints/Flecha_Hielo.Flecha_Hielo_C" (`KismetMathLibrary.MakeTransform` (0.0 0.0 0.0)) "Undefined" "OverrideRootScale" Character "NewEnumerator2" null))
      (bind _output_get (set `self.Flechas` _returnvalue))
      (`self.K2_AttachToComponent` _output_get (`self.Bow`) "Flechas" "KeepRelative" "KeepRelative" "KeepRelative" true))
    (:`else`)))

(fn `UserConstructionScript`)