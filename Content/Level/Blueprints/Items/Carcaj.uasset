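; Quiver pickup that spins continuously about its yaw axis and stands in for an arrow refill.
; When anything overlaps its sphere while off cooldown, it hides the sack and only prints a "+10 arrows" message in Spanish, granting no ammo.
; The cooldown clears and the sack reappears after a five-second delay triggered by end overlap.
; An alternative sine-driven rotation is left unconnected.
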(event `self.ReceiveTick`
  (params (DeltaSeconds :type "Float (single-precision)"))
  (`SceneComponent.K2_AddRelativeRotation` (`self.DefaultSceneRoot`) (`KismetMathLibrary.MakeRotator` 0.0 0.0 (* DeltaSeconds (`self.speedRotation`))) false false))

(event `self.Sphere.OnComponentBeginOverlap`
  (params (OverlappedComponent :type "PrimitiveComponent Object Reference") (OtherActor :type "Actor Object Reference") (OtherComp :type "PrimitiveComponent Object Reference") (OtherBodyIndex :type Integer) (bFromSweep :type Boolean) (SweepResult :type "HitResult Structure (by ref)"))
  (if (not (`self.cooldown`))
    (`SceneComponent.SetVisibility` (`self.sack`) false true)
    (`KismetSystemLibrary.PrintString` "+ 10 flechas")
    (set `self.cooldown` true)))

(event `self.Sphere.OnComponentEndOverlap`
  (params (OverlappedComponent :type "PrimitiveComponent Object Reference") (OtherActor :type "Actor Object Reference") (OtherComp :type "PrimitiveComponent Object Reference") (OtherBodyIndex :type Integer))
  (`KismetSystemLibrary.Delay` 5.0)
  (`SceneComponent.SetVisibility` (`self.sack`) true true)
  (set `self.cooldown` false))

(fn `UserConstructionScript`)